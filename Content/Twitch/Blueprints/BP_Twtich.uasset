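; Twitch chat bridge Blueprint that lets viewers join the game and switch lanes through chat commands.
; On BeginPlay it performs a local Twitch login, requests the channel's feed and registers "join" and "lane" commands.
; Each command handler casts the game instance to BP_MainGI and forwards the sender's name, plus the requested lane, to add players or change lanes.
; Chat and cheer handlers are empty, and login failures only print messages.
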(event Custom|OnChat
  (params (TwitchMessage :type Twitch%20Message%20Structure)))

(event Custom|OnCheer
  (params (TwitchCheer :type Twitch%20Cheer%20Structure)))

(event Custom|JoinGame
  (params (Parameters :type Array%20of%20Strings) (Sender :type Twitch%20Message%20Author%20Structure))
  (bind _asbp_main_gi (Utilities|Casting|CastToBP_MainGI (Game|GetGameInstance)))
  (Default|CallLevelAddPlayers _asbp_main_gi (.name Sender)))

(event Custom|ChangeLane
  (params (Parameters :type Array%20of%20Strings) (Sender :type Twitch%20Message%20Author%20Structure))
  (bind _output (Utilities|Array|Get(acopy) Parameters))
  (bind _asbp_main_gi (Utilities|Casting|CastToBP_MainGI (Game|GetGameInstance)))
  (Development|PrintString (Utilities|String|Append _output (.name Sender)))
  (Default|CallLevelChangeLane _asbp_main_gi (.name Sender) _output))

(event EventBeginPlay
  (bind _credentials (|PerformLocalTwitchLogin)
    (:OnSuccess
      (bind _twitchchat (|RequestFeed (delegate Custom|OnChat) (delegate Custom|OnCheer) _credentials (.Username (Utilities|Struct|BreakTwitchLoginCredentials _credentials)))
        (:OnSuccessfulLogin
          (Variables|Default|SetTwitchChat _twitchchat)
          (Class|TwitchPluginBPLibrary|CreateTwitchCommand (Variables|Default|GetTwitchChat) (Utilities|Struct|MakeTwitchCommandBinding (Utilities|Struct|MakeTwitchCommand "join" "If you wanna join the game, type !join" 0 true) (delegate Custom|JoinGame)))
          (Class|TwitchPluginBPLibrary|CreateTwitchCommand (Variables|Default|GetTwitchChat) (Utilities|Struct|MakeTwitchCommandBinding (Utilities|Struct|MakeTwitchCommand "lane" "Change lane into what you wanna go" (Utilities|Array|MakeArray (Utilities|Struct|MakeTwitchCommandParameter "lane Number" "lane desire to move" " ")) true) (delegate Custom|ChangeLane))))
        (:OnFailedLogin
          (Development|PrintString "Failed Login to Twitch"))))
    (:OnFail
      (Development|PrintString "Login failed"))))

(fn ConstructionScript)