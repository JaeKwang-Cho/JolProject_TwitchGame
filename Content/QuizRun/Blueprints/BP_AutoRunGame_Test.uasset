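; BP_AutoRunGame_Test is a test Blueprint that shows and removes quiz widgets for the QuizRun auto-run game.
; ShowProblems creates a WBP_test widget, stores it as CurQuiz, adds it to the viewport and increments CurProblemNum in BP_MainGI_Test while problems remain in ProblemArray.
; DestroyProblems removes CurQuiz under the same index check, so the last problem's widget is not removed there.
; BeginPlay is empty, and a leftover widget-creation chain is unconnected.
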(event EventBeginPlay)

(fn ConstructionScript)

(fn ShowProblems
  (bind _asbp_main_gi_test (Utilities|Casting|CastToBP_MainGI_Test (Game|GetGameInstance)))
  (if (< (Variables|/Game/QuizRun/Blueprints/BP_MainGI_Test.BP_MainGI_Test_C|GetCurProblemNum _asbp_main_gi_test) (Utilities|Array|Length (Variables|/Game/QuizRun/Blueprints/BP_MainGI_Test.BP_MainGI_Test_C|GetProblemArray _asbp_main_gi_test)))
    (bind _returnvalue (UserInterface|CreateWidget "/Game/UMG/ShowProblem/WBP_test.WBP_test_C" (Game|GetPlayerController 0)))
    (bind _output_get (Variables|Default|SetCurQuiz _returnvalue))
    (UserInterface|Viewport|AddtoViewport _returnvalue 0)
    (bind _asbp_main_gi_test_2 (Utilities|Casting|CastToBP_MainGI_Test (Game|GetGameInstance)))
    (Variables|/Game/QuizRun/Blueprints/BP_MainGI_Test.BP_MainGI_Test_C|SetCurProblemNum _asbp_main_gi_test_2 (+ (Variables|/Game/QuizRun/Blueprints/BP_MainGI_Test.BP_MainGI_Test_C|GetCurProblemNum _asbp_main_gi_test_2) 1))))

(fn DestroyProblems
  (bind _asbp_main_gi_test (Utilities|Casting|CastToBP_MainGI_Test (Game|GetGameInstance)))
  (if (< (Variables|/Game/QuizRun/Blueprints/BP_MainGI_Test.BP_MainGI_Test_C|GetCurProblemNum _asbp_main_gi_test) (Utilities|Array|Length (Variables|/Game/QuizRun/Blueprints/BP_MainGI_Test.BP_MainGI_Test_C|GetProblemArray _asbp_main_gi_test)))
    (Default|Remove (Variables|Default|GetCurQuiz))))