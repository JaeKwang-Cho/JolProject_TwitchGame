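; Test auto-running character for QuizRun that follows a spline's tangent while started, with a random creature color picked at construction.
; Tick drives movement and camera boom and turns the ID nameplate toward the camera.
; TargetLane starts random and changes by keys 1-3 or ChangeLane, but is not applied here.
; StopMoving plays a win animation; Eliminate disables collision, plays lightning shock effects, then notifies the game instance.
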(event Custom|Eliminate
  (bind _capsulecomponent (Variables|Collision|GetCapsuleComponent))
  (bind _returnvalue (Transformation|GetWorldLocation _capsulecomponent))
  ;[1 1 1] Life Management
  (Collision|SetCollisionEnabled (Variables|Collision|GetCapsuleComponent) "NoCollision")
  (Variables|Default|SetStart false)
  (bind _returnvalue_2 (Niagara|SpawnSystematLocation "/Game/QuizRun/Material/NS_Lightning.NS_Lightning" (Math|Vector|MakeVector (.x _returnvalue) (.y _returnvalue) (+ (.z _returnvalue) 5e+02)) "0, 0, 0" "1.000000,1.000000,1.000000" true true "AutoRelease"))
  (bind _returnvalue_3 (Niagara|SpawnSystematLocation "/Game/QuizRun/Material/NS_Shocked.NS_Shocked" (Transformation|GetSocketLocation (Variables|Character|GetMesh) "neck_Socket") "0, 0, 0" "1.000000,1.000000,1.000000" true true "AutoRelease"))
  (Components|Animation|PlayAnimation (Variables|Character|GetMesh) "/Game/CuteCreature/Animations/Anim_ElecShock.Anim_ElecShock" true)
  (Utilities|FlowControl|Delay 1.0)
  (Components|Activation|Deactivate _returnvalue_2)
  (Components|Activation|Deactivate _returnvalue_3)
  (bind _asbp_main_gi_test (Utilities|Casting|CastToBP_MainGI_Test (Game|GetGameInstance)))
  (Default|CallLevelEliminateCaller _asbp_main_gi_test self))

(event Custom|ChangeLane
  (params (Lane :type Integer))
  (Variables|Default|SetTargetLane Lane))

(event Custom|StartMoving
  ;[1 1 1] Life Management
  (Variables|Default|SetStart true))

(event Custom|StopMoving
  ;[1 1 1] Life Management
  (Utilities|FlowControl|Delay (Math|Random|RandomFloatinRange 0.5 1.0))
  (Variables|Default|SetStart false)
  (Components|Animation|PlayAnimation (Variables|Character|GetMesh) "/Game/CuteCreature/Animations/Anim_Win.Anim_Win" true))

(event EventBeginPlay
  ;[1 1 1] NameTag
  (bind _aswbp_name_plate (Utilities|Casting|CastToWBP_NamePlate (UserInterface|GetWidget (Variables|Default|Getnameplate))))
  (Variables|/Game/UMG/WBP_NamePlate.WBP_NamePlate_C|SetID _aswbp_name_plate (Utilities|Text|ToText(String) (Variables|Default|GetID)))
  (Variables|/Game/UMG/WBP_NamePlate.WBP_NamePlate_C|SetNum _aswbp_name_plate (Variables|Default|GetIndex))
  (Variables|Default|SetTargetLane (Math|Random|RandomIntegerinRange 1 3)))

(event EventTick
  (params (DeltaSeconds :type Float%20%28single-precision%29))
  (bind _nameplate (Variables|Default|Getnameplate))
  (bind _capsulecomponent (Variables|Collision|GetCapsuleComponent))
  (bind _curvesplineref (Variables|Default|GetCurveSplineRef))
  (bind _nameplate_2 (Variables|Default|Getnameplate))
  (bind _cameraboom (Variables|Camera|GetCameraBoom))
  (bind _returnvalue (Transformation|GetWorldLocation _capsulecomponent))
  (bind _returnvalue_2 (Transformation|GetWorldLocation _cameraboom))
  (bind _spline (Variables|/Game/QuizRun/Blueprints/BP_Path.BP_Path_C|GetSpline _curvesplineref))
  (bind _returnvalue_3 (Class|SplineComponent|FindTangentClosesttoWorldLocation _spline _returnvalue "World"))
  (bind _returnvalue_4 (Math|Rotator|FindLookatRotation _returnvalue_2 _returnvalue_3))
  (bind (_roll _pitch _yaw) (Math|Rotator|BreakRotator _returnvalue_4))
  ;[1 1 1] Movement
  (if (Variables|Default|GetStart)
    (Pawn|Input|AddMovementInput (Class|SplineComponent|FindTangentClosesttoWorldLocation (Variables|/Game/QuizRun/Blueprints/BP_Path.BP_Path_C|GetSpline (Variables|Default|GetCurveSplineRef)) (Transformation|GetWorldLocation (Variables|Collision|GetCapsuleComponent)) "World") 1.0 false)
    ;[1 0 0] 카메라 효과 어떻게 좀...
    (Transformation|SetRelativeLocation (Variables|Camera|GetCameraBoom) (Math|Vector|MakeVector 1.0 1.0 2e+02) false false)
    (Transformation|SetRelativeRotation (Variables|Camera|GetCameraBoom) (Math|Rotator|MakeRotator _roll -1e+01 (+ _yaw -9e+01)) false false)
    (Transformation|SetWorldRotation _nameplate (Math|Rotator|FindLookatRotation (Transformation|GetWorldLocation _nameplate) (Camera|GetCameraLocation (Game|GetPlayerCameraManager 0))) false false)
    (else
      (Transformation|SetWorldRotation _nameplate_2 (Math|Rotator|FindLookatRotation (Transformation|GetWorldLocation _nameplate_2) (Camera|GetCameraLocation (Game|GetPlayerCameraManager 0))) false false))))

(event Input|KeyboardEvents|3
  (params (Key :type Key%20Structure :default "None"))
  ;[1 1 1] change Lane
  (:Pressed
    (Variables|Default|SetTargetLane 3)))

(event Input|KeyboardEvents|1
  (params (Key :type Key%20Structure :default "None"))
  ;[1 1 1] change Lane
  (:Pressed
    (Variables|Default|SetTargetLane 1)))

(event Input|KeyboardEvents|2
  (params (Key :type Key%20Structure :default "None"))
  ;[1 1 1] change Lane
  (:Pressed
    (Variables|Default|SetTargetLane 2)))

(fn ConstructionScript
  (switch int (Math|Random|RandomIntegerinRange 0 4)
    (:0
      (for _index (range 0 5)
        (Rendering|Material|SetMaterial (Variables|Character|GetMesh) _index "/Game/CuteCreature/Materials/M_CuteCreature_purple.M_CuteCreature_Purple")))
    (:1
      (for _index_2 (range 0 5)
        (Rendering|Material|SetMaterial (Variables|Character|GetMesh) _index_2 "/Game/CuteCreature/Materials/MI_CuteCreature_Black.MI_CuteCreature_Black")))
    (:2
      (for _index_3 (range 0 5)
        (Rendering|Material|SetMaterial (Variables|Character|GetMesh) _index_3 "/Game/CuteCreature/Materials/MI_CuteCreature_Blue.MI_CuteCreature_Blue")))
    (:3
      (for _index_4 (range 0 5)
        (Rendering|Material|SetMaterial (Variables|Character|GetMesh) _index_4 "/Game/CuteCreature/Materials/MI_CuteCreature_Orange.MI_CuteCreature_Orange")))
    (:4
      (for _index_5 (range 0 5)
        (Rendering|Material|SetMaterial (Variables|Character|GetMesh) _index_5 "/Game/CuteCreature/Materials/MI_CuteCreature_Pink.MI_CuteCreature_Pink")))))