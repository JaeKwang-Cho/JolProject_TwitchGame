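; BP_Gates_Test is an answer gate in the quiz runner that judges the auto-running character when it overlaps the gate's box.
; A character whose TargetLane matches the gate's AnswerGate has that lane reset to -1, while any other character is eliminated.
; The first correct pass also has the game mode show problems and destroy them four seconds later, guarded by a DoOnce so it runs only once.
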(event OnComponentBeginOverlap(Box)
  (params (OverlappedComponent :type Primitive%20Component%20Object%20Reference) (OtherActor :type Actor%20Object%20Reference) (OtherComp :type Primitive%20Component%20Object%20Reference) (OtherBodyIndex :type Integer) (bFromSweep :type Boolean) (SweepResult :type Hit%20Result%20Structure%20%28by%20ref%29))
  (bind _asbp_auto_character_test (Utilities|Casting|CastToBP_AutoCharacter_Test OtherActor))
  (if (== (Variables|/Game/QuizRun/Blueprints/BP_AutoCharacter_Test.BP_AutoCharacter_Test_C|GetTargetLane _asbp_auto_character_test) (Variables|Default|GetAnswerGate))
    (Variables|/Game/QuizRun/Blueprints/BP_AutoCharacter_Test.BP_AutoCharacter_Test_C|SetTargetLane _asbp_auto_character_test -1)
    (Utilities|FlowControl|DoOnce false
      (:Completed
        (bind _asbp_auto_run_game_test (Utilities|Casting|CastToBP_AutoRunGame_Test (Game|GetGameMode)))
        (Default|ShowProblems _asbp_auto_run_game_test)
        (Utilities|FlowControl|Delay 4.0)
        (Default|DestroyProblems _asbp_auto_run_game_test)))
    (else
      (Default|Eliminate _asbp_auto_character_test))))

(fn ConstructionScript)