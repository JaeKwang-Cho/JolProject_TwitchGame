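; BP_GatesPoints is a Blueprint in QuizRun that gathers a set of five gate points into a single Points array.
; BeginPlay appends GatePoint1 through GatePoint5 to Points in numeric order, so the array is filled at runtime.
; The construction script is empty, and nothing in this Blueprint's graphs reads the array.
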(event EventBeginPlay
  (bind _points (Variables|Default|GetPoints))
  (Utilities|Array|Add _points (Variables|Default|GetGatePoint1))
  (Utilities|Array|Add _points (Variables|Default|GetGatePoint2))
  (Utilities|Array|Add _points (Variables|Default|GetGatePoint3))
  (Utilities|Array|Add _points (Variables|Default|GetGatePoint4))
  (Utilities|Array|Add _points (Variables|Default|GetGatePoint5)))

(fn ConstructionScript)